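; BP_MonsterSpawn is a spawner that creates BP_Monster_Base actors at its own location and hands each its Spline.
; On BeginPlay it samples the spline every 100 units, skipping the start, into MonsterWalkBlockLocation as world positions.
; A looping one-second timer drives the spawning and is paused after a two-second delay, so only the first brief burst of monsters spawns.
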(event `self.ReceiveBeginPlay`
  (`self.GetMonsterWalkBlockLocation`)
  (bind _returnvalue (`KismetSystemLibrary.K2_SetTimerDelegate` (delegate `SpawnMonster`) 1.0 true -1.0))
  (bind _output_get (set `self.TimerSpawnMonster` _returnvalue))
  (`KismetSystemLibrary.Delay` 2.0)
  (`KismetSystemLibrary.K2_PauseTimerHandle` _output_get))

(event `SpawnMonster`
  (`|SpawnActorFromClass` "/Game/BP/Monster/BP_Monster_Base.BP_Monster_Base_C" (`KismetMathLibrary.Conv_VectorToTransform` (`self.K2_GetActorLocation`)) "AlwaysSpawn" "OverrideRootScale" null (`self.Spline`) null))

(fn `GetMonsterWalkBlockLocation`
  (`KismetArrayLibrary.Array_Clear` (`self.MonsterWalkBlockLocation`))
  (for _index (range 1 (/ (`KismetMathLibrary.FTrunc` (`SplineComponent.GetSplineLength` (`self.Spline`))) 100))
    (`KismetArrayLibrary.Array_Add` (`self.MonsterWalkBlockLocation`) (`SplineComponent.GetLocationAtDistanceAlongSpline` (`self.Spline`) (`KismetMathLibrary.Conv_IntToDouble` (* _index 100)) "World"))))

(fn `UserConstructionScript`)