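; Base monster actor that travels along a spline and costs the player HP on reaching the end.
; Tick advances it by current speed, behind a macro that fires death and destroys it once DestroySelf is set.
; Events apply bullet damage, timed poison and slow, hellfire and healing, routing HP changes through the health component.
; Hit and death events notify components implementing I_MonsterState; BeginPlay adds an HP widget to the viewport.
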(event `self.ReceiveBeginPlay`
  (bind _returnvalue (`|CreateWidget` "/Game/Hud/BP_HP.BP_HP_C" (`GameplayStatics.GetPlayerController` 0) self))
  (bind _output_get (set `self.HPShow` _returnvalue))
  (`UserWidget.AddToViewport` _output_get 0)
  (set `self.NowSpeed` (`self.MaxSpeed`)))

(event `self.ReceiveTick`
  (params (DeltaSeconds :type "Float (single-precision)"))
  (`self.DestroyActor`
    (:`continue`
      (`self.MonsterMove` DeltaSeconds))))

(event `self.PaperSprite.OnComponentBeginOverlap`
  (params (OverlappedComponent :type "PrimitiveComponent Object Reference") (OtherActor :type "Actor Object Reference") (OtherComp :type "PrimitiveComponent Object Reference") (OtherBodyIndex :type Integer) (bFromSweep :type Boolean) (SweepResult :type "HitResult Structure (by ref)")))

(event `self.BulletSingleDamage`
  (params (Damage :type "Float (single-precision)"))
  ;[1 1 1] 受伤
  (`/Game/BP/Monster/Component/BMHP.GetDamage-` (`self.BP_MonsterHealthyComponent`) Damage))

(event `self.BulletPoison`
  (params (Time :type "Float (single-precision)") (Interval :type "Float (single-precision)") (Damage :type "Float (single-precision)"))
  ;[1 1 1] 中毒
  (if (not (`self.bIsPoison`))
    (set `self.bIsPoison` true)
    (bind _returnvalue (`KismetSystemLibrary.K2_SetTimerDelegate` (delegate `PoisonHurt`) Interval true 0.0 (* -1 Interval)))
    (set `self.TPoison` _returnvalue))
  (`KismetSystemLibrary.RetriggerableDelay` Time)
  (`KismetSystemLibrary.K2_PauseTimerHandle` (`self.TPoison`))
  (set `self.bIsPoison` false))

(event `PoisonHurt`
  ;[1 1 1] 中毒
  (`self.DestroyActor`
    (:`continue`
      (`/Game/BP/Monster/Component/BMHP.GetDamage-` (`self.BP_MonsterHealthyComponent`) (stale `self.BulletPoison` Damage)))))

(event `self.BulletLowSpeed`
  (params (LowPercent :type "Float (single-precision)") (Time :type "Float (single-precision)"))
  ;[1 1 1] 减速
  (set `self.NowSpeed` (* LowPercent (`self.MaxSpeed`)))
  (`KismetSystemLibrary.RetriggerableDelay` Time)
  (set `self.NowSpeed` (`self.MaxSpeed`)))

(event `self.MonsterBeHit`
  ;[1 1 1] 被击中时
  (for _array_element (`self.GetComponentsByInterface` "/Game/BP/Monster/Component/I_MonsterState.I_MonsterState_C")
    (message `/Game/BP/Monster/Component/I_MonsterState.Hit` _array_element)))

(event `EventDead`
  (`/Engine/EditorBlueprintResources/StandardMacros.DoOnce` false
    (:`Completed`
      (for _array_element (`self.GetComponentsByInterface` "/Game/BP/Monster/Component/I_MonsterState.I_MonsterState_C")
        (message `/Game/BP/Monster/Component/I_MonsterState.Dead` _array_element)))))

(event `HellFire`
  (params (FireDuration :type "Float (double-precision)") (Damage :type "Float (double-precision)"))
  (if (not (`self.bIsFiring`))
    (`KismetSystemLibrary.PrintString` "fire")
    (set `self.bIsFiring` true)
    (`/Game/BP/Monster/Component/BMHP.GetDamage-` (`self.BP_MonsterHealthyComponent`) Damage)
    (`self.MonsterBeHit`)
    (`KismetSystemLibrary.Delay` FireDuration)
    (set `self.bIsFiring` false)))

(event `Healing`
  (params (HealingHP :type "Float (double-precision)") (HealingInterval :type "Float (double-precision)"))
  (if (not (`self.bIsHealing`))
    (set `self.bIsHealing` true)
    (`/Game/BP/Monster/Component/BMHP.GetDamage-` (`self.BP_MonsterHealthyComponent`) HealingHP)
    (`KismetSystemLibrary.Delay` HealingInterval)
    (set `self.bIsHealing` true)))

(fn `MonsterMove`
  (params (`Delta Time` :type "Float (double-precision)"))
  (bind _spline (`self.Spline`))
  (bind _output_get (set `self.NowDistant` (+ (* `Delta Time` (`self.NowSpeed`)) (`self.NowDistant`))))
  (`self.K2_SetActorLocation` (`SplineComponent.GetLocationAtDistanceAlongSpline` _spline _output_get "World"))
  (if (> _output_get (`SplineComponent.GetSplineLength` _spline))
    (`KismetSystemLibrary.PrintString` "Monster To The End")
    (`/Game/BP/BP_PC.UpdateHP` (cast `/Game/BP/BP_PC` (`GameplayStatics.GetPlayerController` 0) :!pure true) -1)
    (`self.K2_DestroyActor`)))

(fn `UserConstructionScript`)