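; Debuff manager owned by a BP_Monster_Base monster that applies timed poison damage to it.
; BeginPlay caches the owning monster and its health component.
; GetPoisoning starts one looping timer, with a negative start delay cancelling the first interval, that calls GetDamage on the health component.
; Repeat calls restart a Retriggerable Delay instead of stacking timers; when it expires, the timer and poisoned flag are cleared.
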(event `self.ReceiveBeginPlay`
  (bind _asbp_monster_base (cast `/Game/BP/Monster/BP_Monster_Base` (`self.GetOwner`) :!pure true))
  (set `self.BP Monster Healthy Component` (`/Game/BP/Monster/BP_Monster_Base.BP_MonsterHealthyComponent` _asbp_monster_base))
  (set `self.As BP Monster Base` _asbp_monster_base))

(event `GetPoisoning`
  (params (interval :type "Float (double-precision)") (damage :type "Float (double-precision)") (BuffTime :type "Float (double-precision)"))
  (if (not (`self.bIsPoisoning`))
    (set `self.bIsPoisoning` true)
    (bind _returnvalue (`KismetSystemLibrary.K2_SetTimerDelegate` (delegate `Poisoning`) interval true (* -1 interval)))
    (set `self.PoisonTimer` _returnvalue))
  (`KismetSystemLibrary.RetriggerableDelay` BuffTime)
  (`KismetSystemLibrary.K2_ClearAndInvalidateTimerHandle` (`self.PoisonTimer`))
  (set `self.bIsPoisoning` false))

(event `Poisoning`
  (`/Game/BP/Monster/BP_MonsterHealthyComponent.GetDamage-` (`self.BP Monster Healthy Component`) (stale `GetPoisoning` damage)))