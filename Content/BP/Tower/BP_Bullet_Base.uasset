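; Base tower bullet actor that flies along a linear copy of its Parent's spline, taken at BeginPlay.
; Tick advances it by Speed, shrinking damage and sprite scale linearly with distance until MaxDistant.
; Sprite overlap with a live monster notifies components implementing I_BulletComponentHit, then calls MonsterBeHit on it.
; A DestroyActor macro gates tick and overlap on the DestroySelf flag, set once the bullet passes the spline's end.
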(event `self.ReceiveBeginPlay`
  (set `self.NowDamage` (`self.MaxDamage`))
  (`self.SetSpline`))

(event `self.ReceiveTick`
  (params (DeltaSeconds :type "Float (single-precision)"))
  (`self.DestroyActor`
    (:`continue`
      (`self.BulletMove` DeltaSeconds)
      (`self.BulletDamageChange`))))

(event `self.PaperSprite.OnComponentBeginOverlap`
  (params (OverlappedComponent :type "PrimitiveComponent Object Reference") (OtherActor :type "Actor Object Reference") (OtherComp :type "PrimitiveComponent Object Reference") (OtherBodyIndex :type Integer) (bFromSweep :type Boolean) (SweepResult :type "HitResult Structure (by ref)"))
  (`self.DestroyActor`
    (:`continue`
      (bind _asbp_monster_base (cast `/Game/BP/Monster/BP_Monster_Base` OtherActor))
      (bind _output_get (set `self.Target` _asbp_monster_base))
      (`/Engine/EditorBlueprintResources/StandardMacros.IsValid` _output_get
        (:`Is Valid`
          (if (not (`/Game/BP/Monster/BP_Monster_Base.DestroySelf` _output_get))
            (for _array_element (`self.GetComponentsByInterface` "/Game/BP/BulletComponent/I_BulletComponentHit.I_BulletComponentHit_C")
              (message `/Game/BP/BulletComponent/I_BulletComponentHit.Hit` _array_element))
            (`/Game/BP/Monster/BP_Monster_Base.MonsterBeHit` _output_get)))))))

(fn `BulletDamageChange`
  (bind _returnvalue (- 1.0 (/ (`self.NowDistant`) (`self.MaxDistant`))))
  (if (`self.DestroySelf`)
    _
    (elif (<= _returnvalue 0.0)
      (`self.K2_DestroyActor`)
      (else
        (set `self.NowDamage` (* _returnvalue (`self.MaxDamage`)))
        (`SceneComponent.SetWorldScale3D` (`self.PaperSprite`) (`KismetMathLibrary.Conv_DoubleToVector` (* _returnvalue 0.5)))))))

(fn `BulletMove`
  (params (`Delta Time` :type "Float (double-precision)"))
  (bind _output_get (set `self.NowDistant` (+ (* `Delta Time` (`self.Speed`)) (`self.NowDistant`))))
  (bind _spline1 (`self.Spline1`)
    (:`then`
      (`SceneComponent.K2_SetWorldLocation` (`self.PaperSprite`) (`SplineComponent.GetLocationAtDistanceAlongSpline` _spline1 _output_get "World") false false)
      (bind _spline1_2 (`self.Spline1`)
        (:`then`
          (if (> (`self.NowDistant`) (`SplineComponent.GetSplineLength` _spline1_2))
            (set `self.DestroySelf` true)))
        (:`else`)))
    (:`else`)))

(fn `DestroyComponent`
  (params (ComponentClass :type "ActorComponent Class Reference"))
  (for _array_element (`self.K2_GetComponentsByClass` ComponentClass)
    (`ActorComponent.K2_DestroyComponent` _array_element)))

(fn `SetSpline`
  (bind _spline1 (`self.Spline1`))
  (bind _spline (`/Game/BP/Tower/BP_Install_Tower.Spline` (`self.Parent`)))
  (`SplineComponent.ClearSplinePoints` (`self.Spline1`) true)
  (for _index (range (`SplineComponent.GetNumberOfSplinePoints` _spline))
    (`SplineComponent.AddSplinePoint` _spline1 (`SplineComponent.GetLocationAtSplinePoint` _spline _index "World") "World" true)
    (`SplineComponent.SetSplinePointType` _spline1 _index "Linear" true)))

(fn `UserConstructionScript`)

(fn `When BulletOverLap`
  (params (Monster :type "/Game/BP/Monster/BP_Monster_Base Object Reference")))