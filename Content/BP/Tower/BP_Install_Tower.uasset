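; Placeable tower that builds a spline path to the monster route and repeatedly spawns bullets once set down.
; On a valid location, a temporary CBP_PathFinder tests each route block to find the shortest connection from the tower.
; That path is extended backwards along the route to the monster spline location and becomes a linear-point spline.
; A looping cooldown timer spawns BulletClass actors with the tower as Parent.
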(event `self.ReceiveBeginPlay`
  (`parent.ReceiveBeginPlay`)
  (set `self.As BP PC` (cast `/Game/BP/BP_PC` (`GameplayStatics.GetPlayerController` 0) :!pure true))
  (`|ExecutionSequence`))

(event `StartShootCD`
  (bind _shootcd (`self.ShootCD`))
  (bind _returnvalue (`KismetSystemLibrary.K2_SetTimerDelegate` (delegate `Shoot`) _shootcd true (* -1 _shootcd)))
  (set `self.TimerShootCD` _returnvalue))

(event `Shoot`
  (`|SpawnActorFromClass` (`self.BulletClass`) (`self.GetTransform`) "AlwaysSpawn" "OverrideRootScale" null self null))

(fn `ActorSetDown`
  (`parent.ActorSetDown`)
  (`self.StartShootCD`))

(fn `CompareTwoArray`
  (params (index :type Integer))
  (bind _returnvalue (`KismetArrayLibrary.Array_Length` (`self.PathPoint`)))
  (bind _returnvalue_2 (`KismetArrayLibrary.Array_Length` (`PathFinder.PathPoint` (`self.PathFinder`))))
  (if (== _returnvalue_2 0)
    _
    (elif (== _returnvalue 0)
      (set `self.PathPoint` (`PathFinder.PathPoint` (`self.PathFinder`)) :!label _label)
      (set `self.Path Finder Index` index)
      (elif (< _returnvalue_2 _returnvalue)
        (goto _label)))))

(fn `SetLocation`
  (params (NewLocation :type "Vector Structure"))
  (`parent.SetLocation` NewLocation)
  (bind _valid (`/Game/BP/BP_FunctionLibrary.LocationIsValid` (`self.Row`) (`self.Col`)))
  (if _valid
    (`self.SetSplinePath`)
    (else
      (`KismetSystemLibrary.PrintString` "LocationIsUnalid"))))

(fn `SetSplineLocation`
  (params (Points :type "Array of Vector Structure (by ref)"))
  (`SplineComponent.SetSplinePoints` (`self.Spline`) Points "World" true)
  (for (_ _array_index) Points
    (`SplineComponent.SetSplinePointType` (`self.Spline`) _array_index "Linear" true)))

(fn `SetSplinePath`
  (locals (tmp :type "Array of Vector Structure"))
  (bind _path_finder_index (`self.Path Finder Index`))
  (bind _pathpoint (`self.PathPoint`))
  (`KismetArrayLibrary.Array_Clear` (`self.PathPoint`))
  (set `self.Path Finder Index` -1)
  (bind _returnvalue (`|SpawnActorFromClass` "/Game/BP/Install/CBP_PathFinder.CBP_PathFinder_C" (`self.GetTransform`) "AlwaysSpawn" "OverrideRootScale" null null))
  (set `self.PathFinder` _returnvalue)
  ;[1 1 1] 找到塔到怪物行走路线的最短路，
  (bind (_arrayindex _arrayelement) (`/Engine/EditorBlueprintResources/StandardMacros.ReverseForEachLoop` (`/Game/BP/BP_GM.Monster Walk Block Location` (cast `/Game/BP/BP_GM` (`GameplayStatics.GetGameMode`) :!pure true)))
    (:`LoopBody`
      (bind (_row _col) (`/Game/BP/BP_FunctionLibrary.LocationToRowCol` _arrayelement))
      (`/Game/BP/Install/CBP_PathFinder.Init` (`self.PathFinder`) (`self.Row`) (`self.Col`) _row _col)
      (`self.CompareTwoArray` _arrayindex))
    (:`Completed`
      ;[1 1 1] 找到最近的怪物路线的点后，添加从怪物出生点到PathFinderIndex之间的坐标点
      (if (!= _path_finder_index -1)
        (for _index (range (+ _path_finder_index 1))
          (`KismetArrayLibrary.Array_Add` _pathpoint (`|GetArrayItem` (`/Game/BP/BP_GM.Monster Walk Block Location` (cast `/Game/BP/BP_GM` (`GameplayStatics.GetGameMode`) :!pure true)) (- _path_finder_index _index))))
        (`KismetArrayLibrary.Array_Add` _pathpoint (`/Game/BP/BP_GM.MonsterSplineLocation` (cast `/Game/BP/BP_GM` (`GameplayStatics.GetGameMode`) :!pure true)))
        (`self.SetSplineLocation` _pathpoint)
        (`self.K2_DestroyActor` (`self.PathFinder`))
        (else
          (`KismetSystemLibrary.PrintString` "no")
          ;[1 1 1] 找不到则将Spline初始化
          (`self.SetSplineLocation` (`self.PathPoint`))
          (`self.K2_DestroyActor` (`self.PathFinder`)))))))

(fn `UserConstructionScript`
  (`parent.UserConstructionScript`))