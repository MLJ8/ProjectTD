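; BP_HellFire is a timed area skill that lays fire along the monster walk path between Start and End distances.
; On BeginPlay it builds a linear spline from BP_MonsterSpawn's spline endpoints and intervening walk-block points, then adds a spline mesh per segment.
; A looping timer calls HellFire on living monsters whose NowDistant falls within that range, avoiding overlap checks, until the actor destroys itself after Time.
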(event `SetFireParticle`
  (`KismetArrayLibrary.Array_Clear` (`self.Path`))
  (bind _returnvalue (`GameplayStatics.GetActorOfClass` "/Game/BP/BP_MonsterSpawn.BP_MonsterSpawn_C"))
  (set `self.MonsterSpawn` _returnvalue)
  (`self.SetSpline`)
  (`self.SetSplineMesh`))

(event `SetDamage`
  (bind _interval (`self.Interval`))
  (bind _returnvalue (`KismetSystemLibrary.K2_SetTimerDelegate` (delegate `Hurt`) _interval true (* -1 _interval)))
  (set `self.HurtTimer` _returnvalue)
  (`KismetSystemLibrary.Delay` (`self.Time`))
  (`KismetSystemLibrary.K2_ClearAndInvalidateTimerHandle` (`self.HurtTimer`))
  (`self.K2_DestroyActor`))

(event `self.ReceiveBeginPlay`
  (`self.SetFireParticle`)
  (`self.SetDamage`))

(event `Hurt`
  (bind _outactors (`GameplayStatics.GetAllActorsOfClass` "/Game/BP/Monster/BP_Monster_Base.BP_Monster_Base_C"))
  (for _array_element _outactors
    (bind _nowdistant (`/Game/BP/Monster/BP_Monster_Base.NowDistant` _array_element))
    (if (and (>= _nowdistant (`self.Start`)) (<= _nowdistant (`self.End`)))
      (if (not (`/Game/BP/Monster/BP_Monster_Base.DestroySelf` _array_element))
        (`/Game/BP/Monster/BP_Monster_Base.HellFire` _array_element (`self.Interval`) (`self.Damage`))))))

(fn `GetPathLocation`
  (bind _start (`self.Start`))
  (bind _end (`self.End`))
  ;[1 1 1] 加头部点
  (`KismetArrayLibrary.Array_Add` (`self.Path`) (`SplineComponent.GetLocationAtDistanceAlongSpline` (`/Game/BP/BP_MonsterSpawn.Spline` (`self.MonsterSpawn`)) (`self.Start`) "World"))
  ;[1 1 1] 头部点在Index前加上Index点
  (switch `int` (mod (`KismetMathLibrary.FFloor` (/ _start 50.0)) 2) ; 0在点后，1在点前
    (:`0`
      _)
    (:`1`
      (bind _index (`/Game/BP/BP_FunctionLibrary.DistantToIndex` _start))
      (`KismetArrayLibrary.Array_Add` (`self.Path`) (`|GetArrayItem` (`MonsterSpawn.MonsterWalkBlockLocation` (`self.MonsterSpawn`)) _index))))
  ;[1 1 1] 添加中间点
  (bind _index_2 (`/Game/BP/BP_FunctionLibrary.DistantToIndex` (`self.Start`)))
  (bind _index_3 (`/Game/BP/BP_FunctionLibrary.DistantToIndex` (`self.End`)))
  (for _index_4 (range (+ _index_2 1) _index_3)
    (`KismetArrayLibrary.Array_Add` (`self.Path`) (`|GetArrayItem` (`MonsterSpawn.MonsterWalkBlockLocation` (`self.MonsterSpawn`)) _index_4)))
  ;[1 1 1] 尾部点在Index后加上Index点
  (switch `int` (mod (`KismetMathLibrary.FFloor` (/ _end 50.0)) 2) ; 0在点后，1在点前
    (:`0`
      (bind _index_5 (`/Game/BP/BP_FunctionLibrary.DistantToIndex` _end))
      (`KismetArrayLibrary.Array_Add` (`self.Path`) (`|GetArrayItem` (`MonsterSpawn.MonsterWalkBlockLocation` (`self.MonsterSpawn`)) _index_5)))
    (:`1`
      _))
  ;[1 1 1] 加上尾部点
  (`KismetArrayLibrary.Array_Add` (`self.Path`) (`SplineComponent.GetLocationAtDistanceAlongSpline` (`/Game/BP/BP_MonsterSpawn.Spline` (`self.MonsterSpawn`)) (`self.End`) "World")))

(fn `SetSpline`
  (bind _path (`self.Path`))
  (bind _spline (`self.Spline`))
  (`self.GetPathLocation`)
  (`SplineComponent.SetSplinePoints` _spline _path "World" true)
  (for (_ _array_index) _path
    (`SplineComponent.SetSplinePointType` _spline _array_index "Linear" true)))

(fn `SetSplineMesh`
  (bind _spline (`self.Spline`))
  (for _index (range (+ (- (`KismetArrayLibrary.Array_Length` (`self.Path`)) 2) 1))
    (bind _returnvalue (`AddComponent|NODE_AddSplineMeshComponent-0` :`bManualAttachment` true :`RelativeTransform` (`KismetMathLibrary.MakeTransform` (- (`self.K2_GetActorLocation`) (0.0 0.0 30.0)) (struct) (1.0 0.5 0.5))))
    (bind (_location _tangent) (`SplineComponent.GetLocationAndTangentAtSplinePoint` _spline _index "Local"))
    (bind (_location_2 _tangent_2) (`SplineComponent.GetLocationAndTangentAtSplinePoint` _spline (+ _index 1) "Local"))
    ;[1 1 1] delete
    (`SplineMeshComponent.SetStartAndEnd` _returnvalue _location _tangent _location_2 _tangent_2 true)))

(fn `UserConstructionScript`)