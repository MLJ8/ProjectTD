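; Base Blueprint for placeable installations, apparently towers, that sit on a row/column grid.
; Clicking its Box component creates a BP_UI_TowerInfo widget bound to this actor and adds it to the viewport.
; SetLocation moves the actor without sweep, clears PathPoint and derives Row and Col from the new location.
; ActorSetDown flags the installation as set down.
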(event `self.ReceiveBeginPlay`)

(event `self.Box.OnClicked`
  (params (TouchedComponent :type "PrimitiveComponent Object Reference") (ButtonPressed :type "Key Structure"))
  (bind _returnvalue (`|CreateWidget` "/Game/Hud/BP_UI_TowerInfo.BP_UI_TowerInfo_C" (`GameplayStatics.GetPlayerController` 0) self))
  (bind _output_get (set `self.InstallInfo` _returnvalue))
  (`UserWidget.AddToViewport` _output_get 0))

(fn `ActorSetDown`
  (set `self.bIsSetDown` true))

(fn `SetLocation`
  (params (NewLocation :type "Vector Structure"))
  (`self.K2_SetActorLocation` NewLocation)
  (`KismetArrayLibrary.Array_Clear` (`self.PathPoint`))
  (bind (_row _col) (`/Game/BP/BP_FunctionLibrary.LocationToRowCol` NewLocation))
  (set `self.Row` _row)
  (set `self.Col` _col))

(fn `UserConstructionScript`)