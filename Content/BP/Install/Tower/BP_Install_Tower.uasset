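; Installable tower that fires bullets and builds a spline path linking itself to the monster route.
; On relocation, a temporary CBP_PathFinder searches toward each monster walk block, keeping the shortest path.
; That path is extended back along the route to the monster spline location and becomes a linear spline.
; Placement starts a looping cooldown timer, offset to fire immediately, which pauses itself after each bullet spawn.
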(event `self.ReceiveBeginPlay`
  (`parent.ReceiveBeginPlay`)
  (set `self.As BP PC` (cast `/Game/BP/BP_PC` (`GameplayStatics.GetPlayerController` 0) :!pure true))
  (`|ExecutionSequence`))

(event `StartShootCD`
  (bind _shootcd (`self.ShootCD`))
  (bind _returnvalue (`KismetSystemLibrary.K2_SetTimerDelegate` (delegate `Shoot`) _shootcd true (* -1 _shootcd)))
  (set `self.TimerShootCD` _returnvalue))

(event `Shoot`
  (`|SpawnActorFromClass` "/Game/BP/Bullet/BP_Bullet_Base.BP_Bullet_Base_C" (`self.GetTransform`) "AlwaysSpawn" "OverrideRootScale" null self null)
  (`KismetSystemLibrary.K2_PauseTimerHandle` (`self.TimerShootCD`)))

(fn `ActorSetDown`
  (`parent.ActorSetDown`)
  (`self.StartShootCD`))

(fn `CompareTwoArray`
  (params (index :type Integer))
  (bind _returnvalue (`KismetArrayLibrary.Array_Length` (`self.PathPoint`)))
  (bind _returnvalue_2 (`KismetArrayLibrary.Array_Length` (`PathFinder.PathPoint` (`self.PathFinder`))))
  (if (== _returnvalue_2 0)
    _
    (elif (== _returnvalue 0)
      (set `self.PathPoint` (`PathFinder.PathPoint` (`self.PathFinder`)) :!label _label)
      (set `self.Path Finder Index` index)
      (elif (< _returnvalue_2 _returnvalue)
        (goto _label)))))

(fn `SetLocation`
  (params (NewLocation :type "Vector Structure"))
  (`parent.SetLocation` NewLocation)
  (`self.SetSplinePath`))

(fn `SetSplineLocation`
  (params (Points :type "Array of Vector Structure (by ref)"))
  (`SplineComponent.SetSplinePoints` (`self.Spline`) Points "World" true)
  (for (_ _array_index) Points
    (`SplineComponent.SetSplinePointType` (`self.Spline`) _array_index "Linear" true)))

(fn `SetSplinePath`
  (locals (tmp :type "Array of Vector Structure"))
  (bind _pathpoint (`self.PathPoint`))
  (bind _path_finder_index (`self.Path Finder Index`))
  (bind _asbp_gm (cast `/Game/BP/BP_GM` (`GameplayStatics.GetGameMode`) :!pure true))
  (set `self.Path Finder Index` -1)
  (bind _returnvalue (`|SpawnActorFromClass` "/Game/BP/Install/CBP_PathFinder.CBP_PathFinder_C" (`self.GetTransform`) "AlwaysSpawn" "OverrideRootScale" null null))
  (bind _output_get (set `self.PathFinder` _returnvalue))
  (bind (_arrayindex _arrayelement) (`/Engine/EditorBlueprintResources/StandardMacros.ReverseForEachLoop` (`/Game/BP/BP_GM.Monster Walk Block Location` _asbp_gm))
    (:`LoopBody`
      (bind (_row _col) (`/Game/BP/BP_FunctionLibrary.LocationToRowCol` _arrayelement))
      (`/Game/BP/Install/CBP_PathFinder.Init` _output_get (`self.Row`) (`self.Col`) _row _col)
      (`self.CompareTwoArray` _arrayindex))
    (:`Completed`
      ;[1 1 1] 添加从怪物出生点到PathFinderIndex之间的坐标点
      (if (!= _path_finder_index -1)
        (for _index (range (+ _path_finder_index 1))
          (`KismetArrayLibrary.Array_Add` _pathpoint (`|GetArrayItem` (`/Game/BP/BP_GM.Monster Walk Block Location` (cast `/Game/BP/BP_GM` (`GameplayStatics.GetGameMode`) :!pure true)) (- _path_finder_index _index))))
        (`KismetArrayLibrary.Array_Add` _pathpoint (`/Game/BP/BP_GM.MonsterSplineLocation` _asbp_gm))
        (`self.SetSplineLocation` _pathpoint)
        (`self.K2_DestroyActor` (`self.PathFinder`))
        (else
          (`self.K2_DestroyActor` (`self.PathFinder`)))))))

(fn `UserConstructionScript`
  (`parent.UserConstructionScript`))