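; Blueprint function library that maps the mouse cursor to cells on a grid-based building map.
; A Visibility trace along the deprojected cursor ray, with debug drawing left on, yields a hit location that snaps to 100-unit blocks and converts to row and column.
; A separate helper flattens row and column into an index using the column count from the building map referenced by BP_PC.
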(fn `2DToIndex`
  (params (Row :type Integer) (Col :type Integer))
  (returns (Index :type Integer))
  (bind _buildingmapref (`self.GetBuildingMapRef` null))
  (return (+ (* Row (`BuildingMap.MapCol` _buildingmapref)) Col)))

(fn `Get Mouse Location`
  (returns (Location :type "Vector Structure"))
  (bind (_worldlocation _worlddirection) (`PlayerController.DeprojectMousePositionToWorld` (`GameplayStatics.GetPlayerController` null)))
  (bind _outhit (`KismetSystemLibrary.LineTraceSingle` :`Start` _worldlocation :`End` (+ _worldlocation (* _worlddirection 10000.0)) :`TraceChannel` "TraceTypeQuery1" :`DrawDebugType` "ForDuration" :`DrawTime` 3.0))
  (return (`.Location` (`GameplayStatics.BreakHitResult` _outhit))))

(fn `GetBuildingMapRef`
  (returns (BuildingMapRef :type "/Game/BP/BP_BuildingMap Object Reference"))
  (return (`/Game/BP/BP_PC.BuildingMapRef` (cast `/Game/BP/BP_PC` (`GameplayStatics.GetPlayerController` null) :!pure true))))

(fn `GetMouseLocationToBlockIndex`
  (returns (Row :type Integer) (Col :type Integer))
  (bind _location (`self.Get Mouse Location` null))
  (bind _blocklocation (`self.Mouse Location to Block Location Offset` _location))
  (bind (_row _col) (`self.LocationToRowCol` _blocklocation))
  (return _row _col))

(fn `LocationToRowCol`
  (params (Location :type "Vector Structure"))
  (returns (Row :type Integer) (Col :type Integer))
  (return (`KismetMathLibrary.FTrunc` (/ (+ Location_Y 1.0) 100.0)) (`KismetMathLibrary.FTrunc` (/ (+ Location_X 1.0) 100.0))))

(fn `Mouse Location to Block Location Offset`
  (params (MouseLocation :type "Vector Structure"))
  (returns (BlockLocation :type "Vector Structure"))
  (return (`KismetMathLibrary.MakeVector` (`KismetMathLibrary.Conv_IntToDouble` (* (`KismetMathLibrary.FFloor` (/ (+ MouseLocation_X 50.0) 100.0)) 100)) (`KismetMathLibrary.Conv_IntToDouble` (* (`KismetMathLibrary.FFloor` (/ (+ MouseLocation_Y 50.0) 100.0)) 100)) MouseLocation_Z)))