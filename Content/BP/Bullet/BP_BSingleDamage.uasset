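; Bullet component that applies single-target damage to a monster when its Hit event fires.
; It reads the target, damage and armor-piercing (IsAP) state from the owning BP_Bullet_Base, then calls BulletSingleDamage on the target.
; Non-AP bullets, or AP bullets not exceeding target HP, flag themselves for destruction.
; Otherwise the AP bullet survives, resetting current and max damage to damage minus target HP, read after the damage call.
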(event `self.ReceiveBeginPlay`)

(event `/Game/BP/Bullet/I_BulletHit.Hit`
  (bind _nowdamage (`self.NowDamage`))
  (bind _target (`self.Target`))
  (bind _asbp_bullet_base (cast `/Game/BP/Tower/BP_Bullet_Base` (`self.GetOwner`) :!pure true))
  (bind _asbp_bullet_base_2 (cast `/Game/BP/Tower/BP_Bullet_Base` (`self.GetOwner`) :!pure true))
  (`KismetSystemLibrary.PrintString` "SingleDamage")
  (set `self.Target` (`/Game/BP/Tower/BP_Bullet_Base.Target` _asbp_bullet_base))
  (set `self.NowDamage` (`/Game/BP/Tower/BP_Bullet_Base.NowDamage` _asbp_bullet_base))
  (set `self.MaxDamage` (`/Game/BP/Tower/BP_Bullet_Base.MaxDamage` _asbp_bullet_base))
  (set `self.bIsAP` (`/Game/BP/Tower/BP_Bullet_Base.bIsAP` _asbp_bullet_base))
  (if (`self.bIsAP`)
    (if (> (`/Game/BP/Monster/BP_MonsterHealthyComponent.NowHP` (`/Game/BP/Monster/BP_Monster_Base.BP_MonsterHealthyComponent` (`self.Target`))) (`self.NowDamage`))
      (`/Game/BP/Monster/BP_Monster_Base.BulletSingleDamage` _target _nowdamage :!label _label)
      (set `/Game/BP/Tower/BP_Bullet_Base.DestroySelf` true (cast `/Game/BP/Tower/BP_Bullet_Base` (`self.GetOwner`) :!pure true))
      (else
        (`/Game/BP/Monster/BP_Monster_Base.BulletSingleDamage` _target _nowdamage)
        (bind _output_get (set `/Game/BP/Tower/BP_Bullet_Base.MaxDamage` (- (`self.NowDamage`) (`/Game/BP/Monster/BP_MonsterHealthyComponent.NowHP` (`/Game/BP/Monster/BP_Monster_Base.BP_MonsterHealthyComponent` (`self.Target`)))) _asbp_bullet_base_2))
        (set `/Game/BP/Tower/BP_Bullet_Base.NowDamage` _output_get _asbp_bullet_base_2)))
    (else
      (goto _label))))