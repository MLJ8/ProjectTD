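; BP_Bullet_Base is a base bullet actor that travels along its Parent's spline and hits monsters.
; Tick advances it by Speed and scales damage down linearly with distance, destroying it at MaxDistant or the spline's end.
; Sprite overlap with a BP_Monster_Base stores the target and sends HitMessage to the bullet's I_BulletHit components, leaving hit effects to them.
; A DestroySelf check gates both tick and overlap, destroying the bullet when set.
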(event `self.ReceiveBeginPlay`
  (set `self.NowDamage` (`self.MaxDamage`)))

(event `self.ReceiveTick`
  (params (DeltaSeconds :type "Float (single-precision)"))
  (`self.DestroyActor`
    (:`continue`
      (`self.BulletMove` DeltaSeconds)
      (`self.BulletDamageChange`))))

(event `self.PaperSprite.OnComponentBeginOverlap`
  (params (OverlappedComponent :type "PrimitiveComponent Object Reference") (OtherActor :type "Actor Object Reference") (OtherComp :type "PrimitiveComponent Object Reference") (OtherBodyIndex :type Integer) (bFromSweep :type Boolean) (SweepResult :type "HitResult Structure (by ref)"))
  (`self.DestroyActor`
    (:`continue`
      (bind _asbp_monster_base (cast `/Game/BP/Monster/BP_Monster_Base` OtherActor))
      (set `self.Target` _asbp_monster_base)
      (for _array_element (`self.GetComponentsByInterface` "/Game/BP/Bullet/I_BulletHit.I_BulletHit_C")
        (message `/Game/BP/Bullet/I_BulletHit.Hit` _array_element)))))

(fn `BulletDamageChange`
  (bind _returnvalue (- 1.0 (/ (`self.NowDistant`) (`self.MaxDistant`))))
  (if (<= _returnvalue 0.0)
    (`self.K2_DestroyActor`)
    (else
      (set `self.NowDamage` (* _returnvalue (`self.MaxDamage`))))))

(fn `BulletMove`
  (params (`Delta Time` :type "Float (double-precision)"))
  (bind _spline (`/Game/BP/Install/Tower/BP_Install_Tower.Spline` (`self.Parent`)))
  (bind _output_get (set `self.NowDistant` (+ (* `Delta Time` (`self.Speed`)) (`self.NowDistant`))))
  (`self.K2_SetActorLocation` (`SplineComponent.GetLocationAtDistanceAlongSpline` _spline _output_get "World"))
  (if (> _output_get (`SplineComponent.GetSplineLength` _spline))
    (`KismetSystemLibrary.PrintString` "Bullet To The End")
    (`self.K2_DestroyActor`)))

(fn `UserConstructionScript`)

(fn `When BulletOverLap`
  (params (Monster :type "/Game/BP/Monster/BP_Monster_Base Object Reference")))