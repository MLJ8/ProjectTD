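; BP_PC is a player controller that holds the player's Money and HP for a mouse-driven game.
; BeginPlay shows the cursor and sets UI-only input without locking the mouse.
; UpdateMoney and UpdateHP add a passed delta to their value, then call MoneyUpdate and HPUpdate to broadcast the change.
; When HP drops to zero or below, UpdateHP only prints a GameOver string.
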(event `self.ReceiveBeginPlay`
  (set `self.bShowMouseCursor` true)
  (`WidgetBlueprintLibrary.SetInputMode_UIOnlyEx` self null))

(event `Key|LeftMouseButton`
  (params (Key :type "Key Structure")))

(fn `UpdateHP`
  (params (A :type Integer))
  (set `self.HP` (+ A (`self.HP`)))
  (`self.HPUpdate`)
  (if (<= (`self.HP`) 0)
    (`KismetSystemLibrary.PrintString` "GameOver")))

(fn `UpdateMoney`
  (params (GetMoeny :type Integer))
  (set `self.Money` (+ GetMoeny (`self.Money`)))
  (`self.MoneyUpdate`))

(fn `UserConstructionScript`)